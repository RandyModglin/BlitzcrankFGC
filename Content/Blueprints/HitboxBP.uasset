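; Hitbox Blueprint that displays a proximity, strike or hurtbox volume, with a distinct material for each type.
; The SpawnHitbox event switches on HitboxType to set the HitboxDisplay material, then moves the display to HitboxLocation without sweeping and makes it visible.
; The graphs handle only this visual setup, with no overlap or damage logic and an empty construction script.
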(event `SpawnHitbox`
  (switch `HitboxEnum` (`self.hitboxType`)
    (:`HB_Proximity`
      (`PrimitiveComponent.SetMaterial` (`self.HitboxDisplay`) 0 "/Game/Art/Materials/Hitboxes/ProximityHB_Mat.ProximityHB_Mat"))
    (:`HB_Strike`
      (`PrimitiveComponent.SetMaterial` (`self.HitboxDisplay`) 0 "/Game/Art/Materials/Hitboxes/HitHB_Mat.HitHB_Mat"))
    (:`HB_Hurtbox`
      (`PrimitiveComponent.SetMaterial` (`self.HitboxDisplay`) 0 "/Game/Art/Materials/Hitboxes/HurtHB_Mat.HurtHB_Mat")))
  (`SceneComponent.K2_SetWorldLocation` (`self.HitboxDisplay`) (`self.hitboxLocation`) false false)
  (`SceneComponent.SetVisibility` (`self.HitboxDisplay`) true false))

(fn `UserConstructionScript`)