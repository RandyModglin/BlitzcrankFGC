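; Default game mode that spawns the Blitzcrank player character and a dummy at tagged PlayerStart actors.
; On BeginPlay it runs SpawnPlayer for every PlayerStart in the level.
; Starts tagged "Player" spawn a BlitzcrankBP that player controller 0 possesses, while those tagged "Dummy" spawn a DummyBP.
; Each spawned pawn takes its start's transform and owner, and is stored in the Player or Dummy variable.
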(event `self.ReceiveBeginPlay`
  (bind _outactors (`GameplayStatics.GetAllActorsOfClass` "/Script/Engine.PlayerStart"))
  (for _array_element _outactors
    (`self.SpawnPlayer` _array_element)))

(fn `SpawnPlayer`
  (params (Object :type "Actor Object Reference"))
  (bind _asplayer_start (cast `PlayerStart` Object))
  (bind _playerstarttag (`PlayerStart.PlayerStartTag` _asplayer_start))
  (if (== "Player" _playerstarttag)
    (bind _returnvalue (`|SpawnActorFromClass` "/Game/Blueprints/BlitzcrankBP.BlitzcrankBP_C" (`self.GetTransform` Object) "Undefined" "OverrideRootScale" Object null))
    (bind _output_get (set `self.Player` _returnvalue))
    (`Controller.Possess` (`GameplayStatics.GetPlayerController` 0) _output_get)
    (elif (== _playerstarttag "Dummy")
      (bind _returnvalue_2 (`|SpawnActorFromClass` "/Game/Blueprints/DummyBP.DummyBP_C" (`self.GetTransform` Object) "Undefined" "OverrideRootScale" Object null))
      (set `self.Dummy` _returnvalue_2))))

(fn `UserConstructionScript`)