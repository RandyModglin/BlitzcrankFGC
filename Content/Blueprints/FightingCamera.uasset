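; Fighting-game camera that keeps the Player and Dummy framed and creates the stage's side walls.
; After a short BeginPlay delay, it takes both fighters from DefaultGameModeBP, spawns two StageWalls outside their positions and stores outer Y limits.
; Each tick it keeps its X, follows their Y midpoint and a scaled Z average, and zooms by setting a clamped FOV from their horizontal separation.
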(event `self.ReceiveBeginPlay`
  (`KismetSystemLibrary.Delay` 0.03)
  (bind _asdefault_game_mode_bp (cast `/Game/Blueprints/DefaultGameModeBP` (`GameplayStatics.GetGameMode`)))
  (bind _player (`BlitzcrankFGCGameMode.Player` _asdefault_game_mode_bp))
  (`/Engine/EditorBlueprintResources/StandardMacros.IsValid` _player
    (:`Is Valid`
      (set `self.playerRef` _player)
      (bind _dummy (`BlitzcrankFGCGameMode.Dummy` _asdefault_game_mode_bp))
      (`/Engine/EditorBlueprintResources/StandardMacros.IsValid` _dummy
        (:`Is Valid`
          (set `self.dummyRef` _dummy)
          (bind _returnvalue (`|SpawnActorFromClass` "/Game/Blueprints/StageWall.StageWall_C" (`self.GetTransform`) "Undefined" "OverrideRootScale" null null))
          (set `self.LeftStageWall` _returnvalue)
          (bind _returnvalue_2 (`|SpawnActorFromClass` "/Game/Blueprints/StageWall.StageWall_C" (`self.GetTransform`) "Undefined" "OverrideRootScale" null null))
          (set `self.RightStageWall` _returnvalue_2)
          (`self.SetStageBoundaries`))))))

(event `self.ReceiveTick`
  (params (DeltaSeconds :type "Float (single-precision)"))
  (bind _playerref (`self.playerRef`))
  (bind _dummyref (`self.dummyRef`))
  (if (and (`KismetSystemLibrary.IsValid` _playerref) (`KismetSystemLibrary.IsValid` _dummyref))
    (`self.K2_SetActorLocation` (`KismetMathLibrary.MakeVector` (.x (`self.K2_GetActorLocation`)) (/ (+ (.y (`self.K2_GetActorLocation` _playerref)) (.y (`self.K2_GetActorLocation` _dummyref))) 2.0) (/ (+ (.z (`self.K2_GetActorLocation` _playerref)) (.z (`self.K2_GetActorLocation` _dummyref))) 1.7)))
    (`CameraComponent.SetFieldOfView` (`self.CameraComponent`) (`KismetMathLibrary.FClamp` (`KismetMathLibrary.Abs` (* (- (.y (`self.K2_GetActorLocation` (`self.playerRef`))) (.y (`self.K2_GetActorLocation` (`self.dummyRef`)))) 0.15)) 60.0 85.0))))

(fn `SetStageBoundaries`
  (bind _returnvalue (- (.y (`self.K2_GetActorLocation` (`self.playerRef`))) 500.0))
  (bind _returnvalue_2 (+ (.y (`self.K2_GetActorLocation` (`self.dummyRef`))) 500.0))
  (set `self.LeftMax` (- _returnvalue 300.0))
  (`self.K2_SetActorLocation` (`self.LeftStageWall`) (`KismetMathLibrary.MakeVector` (.x (`self.K2_GetActorLocation` (`self.playerRef`))) _returnvalue (.z (`self.K2_GetActorLocation` (`self.playerRef`)))) false false)
  (set `self.RightMax` (+ _returnvalue_2 300.0))
  (`self.K2_SetActorLocation` (`self.RightStageWall`) (`KismetMathLibrary.MakeVector` (.x (`self.K2_GetActorLocation` (`self.dummyRef`))) _returnvalue_2 (.z (`self.K2_GetActorLocation` (`self.dummyRef`)))) false false))

(fn `UserConstructionScript`)